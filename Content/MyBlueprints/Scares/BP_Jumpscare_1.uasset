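; BP_Jumpscare_1 is a one-shot jumpscare triggered when the player enters its Box volume.
; It caches the first-person player character on BeginPlay and compares it against the overlapping actor.
; On the first matching overlap, a DoOnce gate activates the InterpToMovement component and plays a 2D scare sound.
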(event `self.ReceiveBeginPlay`
  (bind _asbp_first_person_character (cast `/Game/FirstPerson/Blueprints/BP_FirstPersonCharacter` (`GameplayStatics.GetPlayerCharacter` 0)))
  (set `self.As BP First Person Character` _asbp_first_person_character))

(event `self.Box.OnComponentBeginOverlap`
  (params (OverlappedComponent :type "PrimitiveComponent Object Reference") (OtherActor :type "Actor Object Reference") (OtherComp :type "PrimitiveComponent Object Reference") (OtherBodyIndex :type Integer) (bFromSweep :type Boolean) (SweepResult :type "HitResult Structure (by ref)"))
  (if (== OtherActor (`self.As BP First Person Character`))
    (`/Engine/EditorBlueprintResources/StandardMacros.DoOnce` false
      (:`Completed`
        (`ActorComponent.Activate` (`self.InterpToMovement`) false)
        (`GameplayStatics.PlaySound2D` "/Game/Bubble_Factory_Game_Audio/SFX/Jump_Scares/jump_scare_2.jump_scare_2" 1.0 1.0 0.0 null null)))))

(fn `UserConstructionScript`)